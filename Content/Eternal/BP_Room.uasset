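; BP_Room is a room actor that drives room streaming around the player through trigger boxes on three hallways, HW2 to HW4.
; When BP_FirstPersonCharacter leaves a hallway's first trigger, it calls DeloadRooms on the character, then SpawnRooms with that hallway's arrow.
; Leaving a hallway's second trigger calls ReloadRooms.
; The room only forwards end-overlap events, as the loading logic lives in the character.
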(event OnComponentEndOverlap(HW2_TriggerBox)
  (params (OverlappedComponent :type Primitive%20Component%20Object%20Reference) (OtherActor :type Actor%20Object%20Reference) (OtherComp :type Primitive%20Component%20Object%20Reference) (OtherBodyIndex :type Integer))
  (bind _asbp_first_person_character (Utilities|Casting|CastToBP_FirstPersonCharacter OtherActor))
  (Default|DeloadRooms _asbp_first_person_character "BP_Room_C")
  (Default|SpawnRooms _asbp_first_person_character _asbp_first_person_character (Variables|Default|GetHW2_Arrow)))

(event OnComponentEndOverlap(HW3_TriggerBox)
  (params (OverlappedComponent :type Primitive%20Component%20Object%20Reference) (OtherActor :type Actor%20Object%20Reference) (OtherComp :type Primitive%20Component%20Object%20Reference) (OtherBodyIndex :type Integer))
  (bind _asbp_first_person_character (Utilities|Casting|CastToBP_FirstPersonCharacter OtherActor))
  (Default|DeloadRooms _asbp_first_person_character "BP_Room_C")
  (Default|SpawnRooms _asbp_first_person_character _asbp_first_person_character (Variables|Default|GetHW3_Arrow)))

(event OnComponentEndOverlap(HW4_TriggerBox)
  (params (OverlappedComponent :type Primitive%20Component%20Object%20Reference) (OtherActor :type Actor%20Object%20Reference) (OtherComp :type Primitive%20Component%20Object%20Reference) (OtherBodyIndex :type Integer))
  (bind _asbp_first_person_character (Utilities|Casting|CastToBP_FirstPersonCharacter OtherActor))
  (Default|DeloadRooms _asbp_first_person_character "BP_Room_C")
  (Default|SpawnRooms _asbp_first_person_character _asbp_first_person_character (Variables|Default|GetHW4_Arrow)))

(event OnComponentEndOverlap(HW2_TriggerBox1)
  (params (OverlappedComponent :type Primitive%20Component%20Object%20Reference) (OtherActor :type Actor%20Object%20Reference) (OtherComp :type Primitive%20Component%20Object%20Reference) (OtherBodyIndex :type Integer))
  (bind _asbp_first_person_character (Utilities|Casting|CastToBP_FirstPersonCharacter OtherActor))
  (Default|ReloadRooms _asbp_first_person_character))

(event OnComponentEndOverlap(HW3_TriggerBox1)
  (params (OverlappedComponent :type Primitive%20Component%20Object%20Reference) (OtherActor :type Actor%20Object%20Reference) (OtherComp :type Primitive%20Component%20Object%20Reference) (OtherBodyIndex :type Integer))
  (bind _asbp_first_person_character (Utilities|Casting|CastToBP_FirstPersonCharacter OtherActor))
  (Default|ReloadRooms _asbp_first_person_character))

(event OnComponentEndOverlap(HW4_TriggerBox1)
  (params (OverlappedComponent :type Primitive%20Component%20Object%20Reference) (OtherActor :type Actor%20Object%20Reference) (OtherComp :type Primitive%20Component%20Object%20Reference) (OtherBodyIndex :type Integer))
  (bind _asbp_first_person_character (Utilities|Casting|CastToBP_FirstPersonCharacter OtherActor))
  (Default|ReloadRooms _asbp_first_person_character))

(event EventBeginPlay)

(event Collision|EventActorBeginOverlap
  (params (OtherActor :type Actor%20Object%20Reference)))

(event EventTick
  (params (DeltaSeconds :type Float%20%28single-precision%29)))

(fn ConstructionScript)