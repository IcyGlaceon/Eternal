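; Room actor that drives streaming of connected rooms as the player leaves hallway trigger boxes, delegating all room management to BP_FirstPersonCharacter.
; Exiting the first trigger in hallways 2–4 spawns rooms at that hallway's arrow, deloads early rooms, disables itself and passes the second to AddCollision.
; Second triggers reload rooms and pass on the third, which respawns rooms relative to this one.
; Hallway 1 only reloads rooms.
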(event OnComponentEndOverlap(HW1_TriggerBox1)
  (params (OverlappedComponent :type Primitive%20Component%20Object%20Reference) (OtherActor :type Actor%20Object%20Reference) (OtherComp :type Primitive%20Component%20Object%20Reference) (OtherBodyIndex :type Integer))
  (bind _asbp_first_person_character (Utilities|Casting|CastToBP_FirstPersonCharacter OtherActor))
  (Default|ReloadRooms _asbp_first_person_character))

(event OnComponentEndOverlap(HW2_TriggerBox2)
  (params (OverlappedComponent :type Primitive%20Component%20Object%20Reference) (OtherActor :type Actor%20Object%20Reference) (OtherComp :type Primitive%20Component%20Object%20Reference) (OtherBodyIndex :type Integer))
  (bind _asbp_first_person_character (Utilities|Casting|CastToBP_FirstPersonCharacter OtherActor))
  (Default|RespawnRooms _asbp_first_person_character _asbp_first_person_character self))

(event OnComponentEndOverlap(HW3_TriggerBox2)
  (params (OverlappedComponent :type Primitive%20Component%20Object%20Reference) (OtherActor :type Actor%20Object%20Reference) (OtherComp :type Primitive%20Component%20Object%20Reference) (OtherBodyIndex :type Integer))
  (bind _asbp_first_person_character (Utilities|Casting|CastToBP_FirstPersonCharacter OtherActor))
  (Default|RespawnRooms _asbp_first_person_character _asbp_first_person_character self))

(event OnComponentEndOverlap(HW2_TriggerBox)
  (params (OverlappedComponent :type Primitive%20Component%20Object%20Reference) (OtherActor :type Actor%20Object%20Reference) (OtherComp :type Primitive%20Component%20Object%20Reference) (OtherBodyIndex :type Integer))
  (bind _asbp_first_person_character (Utilities|Casting|CastToBP_FirstPersonCharacter OtherActor))
  (bind _currentroom (Default|SpawnRooms _asbp_first_person_character _asbp_first_person_character (Variables|Default|GetHW2_Arrow)))
  (Default|DeloadEarlyRooms _asbp_first_person_character _currentroom)
  (Collision|SetCollisionEnabled (Variables|Default|GetHW2_TriggerBox) "NoCollision")
  (Default|AddCollision _asbp_first_person_character (Variables|Default|GetHW2_TriggerBox1)))

(event OnComponentEndOverlap(HW3_TriggerBox)
  (params (OverlappedComponent :type Primitive%20Component%20Object%20Reference) (OtherActor :type Actor%20Object%20Reference) (OtherComp :type Primitive%20Component%20Object%20Reference) (OtherBodyIndex :type Integer))
  (bind _asbp_first_person_character (Utilities|Casting|CastToBP_FirstPersonCharacter OtherActor))
  (bind _currentroom (Default|SpawnRooms _asbp_first_person_character _asbp_first_person_character (Variables|Default|GetHW3_Arrow)))
  (Default|DeloadEarlyRooms _asbp_first_person_character _currentroom)
  (Collision|SetCollisionEnabled (Variables|Default|GetHW3_TriggerBox) "NoCollision")
  (Default|AddCollision _asbp_first_person_character (Variables|Default|GetHW3_TriggerBox1)))

(event OnComponentEndOverlap(HW4_TriggerBox)
  (params (OverlappedComponent :type Primitive%20Component%20Object%20Reference) (OtherActor :type Actor%20Object%20Reference) (OtherComp :type Primitive%20Component%20Object%20Reference) (OtherBodyIndex :type Integer))
  (bind _asbp_first_person_character (Utilities|Casting|CastToBP_FirstPersonCharacter OtherActor))
  (bind _currentroom (Default|SpawnRooms _asbp_first_person_character _asbp_first_person_character (Variables|Default|GetHW4_Arrow)))
  (Default|DeloadEarlyRooms _asbp_first_person_character _currentroom)
  (Collision|SetCollisionEnabled (Variables|Default|GetHW4_TriggerBox) "NoCollision")
  (Default|AddCollision _asbp_first_person_character (Variables|Default|GetHW4_TriggerBox1)))

(event OnComponentEndOverlap(HW2_TriggerBox1)
  (params (OverlappedComponent :type Primitive%20Component%20Object%20Reference) (OtherActor :type Actor%20Object%20Reference) (OtherComp :type Primitive%20Component%20Object%20Reference) (OtherBodyIndex :type Integer))
  (bind _asbp_first_person_character (Utilities|Casting|CastToBP_FirstPersonCharacter OtherActor))
  (Default|ReloadRooms _asbp_first_person_character)
  (Default|AddCollision _asbp_first_person_character (Variables|Default|GetHW2_TriggerBox2)))

(event OnComponentEndOverlap(HW3_TriggerBox1)
  (params (OverlappedComponent :type Primitive%20Component%20Object%20Reference) (OtherActor :type Actor%20Object%20Reference) (OtherComp :type Primitive%20Component%20Object%20Reference) (OtherBodyIndex :type Integer))
  (bind _asbp_first_person_character (Utilities|Casting|CastToBP_FirstPersonCharacter OtherActor))
  (Default|ReloadRooms _asbp_first_person_character)
  (Default|AddCollision _asbp_first_person_character (Variables|Default|GetHW3_TriggerBox2)))

(event OnComponentEndOverlap(HW4_TriggerBox1)
  (params (OverlappedComponent :type Primitive%20Component%20Object%20Reference) (OtherActor :type Actor%20Object%20Reference) (OtherComp :type Primitive%20Component%20Object%20Reference) (OtherBodyIndex :type Integer))
  (bind _asbp_first_person_character (Utilities|Casting|CastToBP_FirstPersonCharacter OtherActor))
  (Default|ReloadRooms _asbp_first_person_character)
  (Default|AddCollision _asbp_first_person_character (Variables|Default|GetHW4_TriggerBox2)))

(event OnComponentEndOverlap(HW4_TriggerBox2)
  (params (OverlappedComponent :type Primitive%20Component%20Object%20Reference) (OtherActor :type Actor%20Object%20Reference) (OtherComp :type Primitive%20Component%20Object%20Reference) (OtherBodyIndex :type Integer))
  (bind _asbp_first_person_character (Utilities|Casting|CastToBP_FirstPersonCharacter OtherActor))
  (Default|RespawnRooms _asbp_first_person_character _asbp_first_person_character self))

(event EventBeginPlay)

(event Collision|EventActorBeginOverlap
  (params (OtherActor :type Actor%20Object%20Reference)))

(event EventTick
  (params (DeltaSeconds :type Float%20%28single-precision%29)))

(fn ConstructionScript)