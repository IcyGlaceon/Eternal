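; BP_KeyRoom is a room actor whose hallway triggers drive room spawning, deloading and reloading through BP_FirstPersonCharacter.
; When the character exits the first trigger, it spawns rooms at the room's Arrow, passes the result to DeloadRooms, disables that trigger and calls AddCollision on the second.
; Exiting the second trigger calls ReloadRooms; an AddCollision call for the first trigger is left unconnected.
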(event OnComponentEndOverlap(Hallway_TriggerBox)
  (params (OverlappedComponent :type Primitive%20Component%20Object%20Reference) (OtherActor :type Actor%20Object%20Reference) (OtherComp :type Primitive%20Component%20Object%20Reference) (OtherBodyIndex :type Integer))
  (bind _asbp_first_person_character (Utilities|Casting|CastToBP_FirstPersonCharacter OtherActor))
  (bind _currentroom (Default|SpawnRooms _asbp_first_person_character _asbp_first_person_character (Variables|Default|GetArrow)))
  (Default|DeloadRooms _asbp_first_person_character _currentroom)
  (Collision|SetCollisionEnabled (Variables|Default|GetHallway_TriggerBox) "NoCollision")
  (Default|AddCollision _asbp_first_person_character (Variables|Default|GetHallway_TriggerBox1)))

(event OnComponentEndOverlap(Hallway_TriggerBox1)
  (params (OverlappedComponent :type Primitive%20Component%20Object%20Reference) (OtherActor :type Actor%20Object%20Reference) (OtherComp :type Primitive%20Component%20Object%20Reference) (OtherBodyIndex :type Integer))
  (bind _asbp_first_person_character (Utilities|Casting|CastToBP_FirstPersonCharacter OtherActor))
  (Default|ReloadRooms _asbp_first_person_character))

(event EventBeginPlay)

(fn ConstructionScript)