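; Small hallway room actor that spawns four puzzle actors at marker components on BeginPlay and drives room streaming around the player.
; Three trigger boxes react when the first-person character leaves them, delegating room management to that character.
; The first spawns rooms from an arrow, deloads early ones and disables itself; the second reloads rooms; the third respawns them relative to this hallway.
; The first two pass the next trigger to the character's AddCollision, chaining the sequence.
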(event OnComponentEndOverlap(Hallway_TriggerBox)
  (params (OverlappedComponent :type Primitive%20Component%20Object%20Reference) (OtherActor :type Actor%20Object%20Reference) (OtherComp :type Primitive%20Component%20Object%20Reference) (OtherBodyIndex :type Integer))
  (bind _asbp_first_person_character (Utilities|Casting|CastToBP_FirstPersonCharacter OtherActor))
  (bind _currentroom (Default|SpawnRooms _asbp_first_person_character _asbp_first_person_character (Variables|Default|GetArrow)))
  (Default|DeloadEarlyRooms _asbp_first_person_character _currentroom)
  (Collision|SetCollisionEnabled (Variables|Default|GetHallway_TriggerBox) "NoCollision")
  (Default|AddCollision _asbp_first_person_character (Variables|Default|GetHallway_TriggerBox1)))

(event OnComponentEndOverlap(Hallway_TriggerBox1)
  (params (OverlappedComponent :type Primitive%20Component%20Object%20Reference) (OtherActor :type Actor%20Object%20Reference) (OtherComp :type Primitive%20Component%20Object%20Reference) (OtherBodyIndex :type Integer))
  (bind _asbp_first_person_character (Utilities|Casting|CastToBP_FirstPersonCharacter OtherActor))
  (Default|ReloadRooms _asbp_first_person_character)
  (Default|AddCollision _asbp_first_person_character (Variables|Default|GetHallway_TriggerBox2)))

(event OnComponentEndOverlap(Hallway_TriggerBox2)
  (params (OverlappedComponent :type Primitive%20Component%20Object%20Reference) (OtherActor :type Actor%20Object%20Reference) (OtherComp :type Primitive%20Component%20Object%20Reference) (OtherBodyIndex :type Integer))
  (bind _asbp_first_person_character (Utilities|Casting|CastToBP_FirstPersonCharacter OtherActor))
  (Default|RespawnRooms _asbp_first_person_character _asbp_first_person_character self))

(event EventBeginPlay
  (bind _spawn_transform_scale (Variables|Default|GetSpawn%20Transform%20Scale))
  (Game|SpawnActorfromClass "/Game/Eternal/Puzzles/SequencePuzzle/BP_Puzzle1.BP_Puzzle1_C" (Math|Transform|MakeTransform (Transformation|GetWorldLocation (Variables|Default|GetPuzzle1)) "0, 0, 0" _spawn_transform_scale) "Undefined" "MultiplyWithRoot" 0 0)
  (Game|SpawnActorfromClass "/Game/Eternal/Puzzles/SequencePuzzle/BP_Puzzle2.BP_Puzzle2_C" (Math|Transform|MakeTransform (Transformation|GetWorldLocation (Variables|Default|GetPuzzle2)) "0, 0, 0" _spawn_transform_scale) "Undefined" "MultiplyWithRoot" 0 0)
  (Game|SpawnActorfromClass "/Game/Eternal/Puzzles/SequencePuzzle/BP_Puzzle3.BP_Puzzle3_C" (Math|Transform|MakeTransform (Transformation|GetWorldLocation (Variables|Default|GetPuzzle3)) "0, 0, 0" _spawn_transform_scale) "Undefined" "MultiplyWithRoot" 0 0)
  (Game|SpawnActorfromClass "/Game/Eternal/Puzzles/SequencePuzzle/BP_Puzzle4.BP_Puzzle4_C" (Math|Transform|MakeTransform (Transformation|GetWorldLocation (Variables|Default|GetPuzzle4)) "0, 0, 0" _spawn_transform_scale) "Undefined" "MultiplyWithRoot" 0 0))

(fn ConstructionScript)