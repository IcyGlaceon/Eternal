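; Starting room actor that hands off to the first-person character's room spawning and removes itself later.
; When the character leaves the Box, it calls the character's SpawnRooms at the Arrow, passes the result to DeloadRooms, then disables Box collision.
; Tick destroys the room once AllRooms holds four entries, taking the character from the OtherActor pin of the empty ActorBeginOverlap event.
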(event OnComponentEndOverlap(Box)
  (params (OverlappedComponent :type Primitive%20Component%20Object%20Reference) (OtherActor :type Actor%20Object%20Reference) (OtherComp :type Primitive%20Component%20Object%20Reference) (OtherBodyIndex :type Integer))
  (bind _asbp_first_person_character (Utilities|Casting|CastToBP_FirstPersonCharacter OtherActor))
  (bind _currentroom (Default|SpawnRooms _asbp_first_person_character _asbp_first_person_character (Variables|Default|GetArrow)))
  (Default|DeloadRooms _asbp_first_person_character _currentroom)
  (Collision|SetCollisionEnabled (Variables|Default|GetBox) "NoCollision"))

(event EventBeginPlay)

(event Collision|EventActorBeginOverlap
  (params (OtherActor :type Actor%20Object%20Reference)))

(event EventTick
  (params (DeltaSeconds :type Float%20%28single-precision%29))
  (bind _asbp_first_person_character (Utilities|Casting|CastToBP_FirstPersonCharacter (stale Collision|EventActorBeginOverlap OtherActor)))
  (if (== (Utilities|Array|Length (Variables|/Game/FirstPerson/Blueprints/BP_FirstPersonCharacter.BP_FirstPersonCharacter_C|GetAllRooms _asbp_first_person_character)) 4)
    (Actor|DestroyActor)))

(fn ConstructionScript)