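; BP_EndRoom is an end room gated by the player's red key.
; On BeginPlay, if the Player reference lacks an active red key, it spawns a BP_KeyDoor at the W component's location and rotation and stores it in KDoor.
; When a first-person character with the red key overlaps the Box trigger, it only prints "End" as the ending response.
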(event OnComponentBeginOverlap(Box)
  (params (OverlappedComponent :type Primitive%20Component%20Object%20Reference) (OtherActor :type Actor%20Object%20Reference) (OtherComp :type Primitive%20Component%20Object%20Reference) (OtherBodyIndex :type Integer) (bFromSweep :type Boolean) (SweepResult :type Hit%20Result%20Structure%20%28by%20ref%29))
  (bind _asbp_first_person_character (Utilities|Casting|CastToBP_FirstPersonCharacter OtherActor))
  (if (Variables|/Game/FirstPerson/Blueprints/BP_FirstPersonCharacter.BP_FirstPersonCharacter_C|GetRedKeyActive _asbp_first_person_character)
    (Development|PrintString "End")))

(event EventBeginPlay
  (bind _w (Variables|Default|Getw))
  (if (not (Variables|/Game/FirstPerson/Blueprints/BP_FirstPersonCharacter.BP_FirstPersonCharacter_C|GetRedKeyActive (Variables|Default|GetPlayer)))
    (bind _returnvalue (Game|SpawnActorfromClass "/Game/Eternal/BP_KeyDoor.BP_KeyDoor_C" (Math|Transform|MakeTransform (Transformation|GetWorldLocation _w) (Transformation|GetWorldRotation _w) "1.000000,1.000000,1.000000") "Undefined" "MultiplyWithRoot" 0 0))
    (Variables|Default|SetKDoor _returnvalue)))

(event Collision|EventActorBeginOverlap
  (params (OtherActor :type Actor%20Object%20Reference)))

(event EventTick
  (params (DeltaSeconds :type Float%20%28single-precision%29)))

(fn ConstructionScript)