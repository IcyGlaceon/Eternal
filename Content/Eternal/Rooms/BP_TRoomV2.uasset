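; T-room segment for a room system that spawns and unloads rooms as the first-person player moves through it.
; Leaving either primary exit box asks the character to spawn rooms from that branch's arrow and deload earlier ones, disables the box and arms its return box.
; Return boxes reload rooms, and the first two arm secondary exit boxes that respawn rooms relative to this one.
; All room logic lives on the character.
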(event OnComponentEndOverlap(BoxExit_1)
  (params (OverlappedComponent :type Primitive%20Component%20Object%20Reference) (OtherActor :type Actor%20Object%20Reference) (OtherComp :type Primitive%20Component%20Object%20Reference) (OtherBodyIndex :type Integer))
  (bind _asbp_first_person_character (Utilities|Casting|CastToBP_FirstPersonCharacter OtherActor))
  (bind _currentroom (Default|SpawnRooms _asbp_first_person_character _asbp_first_person_character (Variables|Default|GetArrow)))
  (Default|DeloadEarlyRooms _asbp_first_person_character _currentroom)
  (Default|AddCollision _asbp_first_person_character (Variables|Default|GetBoxReturn_1))
  (Collision|SetCollisionEnabled (Variables|Default|GetBoxExit_1) "NoCollision"))

(event OnComponentEndOverlap(BoxExit_2)
  (params (OverlappedComponent :type Primitive%20Component%20Object%20Reference) (OtherActor :type Actor%20Object%20Reference) (OtherComp :type Primitive%20Component%20Object%20Reference) (OtherBodyIndex :type Integer))
  (bind _asbp_first_person_character (Utilities|Casting|CastToBP_FirstPersonCharacter OtherActor))
  (bind _currentroom (Default|SpawnRooms _asbp_first_person_character _asbp_first_person_character (Variables|Default|GetArrow1)))
  (Default|DeloadEarlyRooms _asbp_first_person_character _currentroom)
  (Collision|SetCollisionEnabled (Variables|Default|GetBoxExit_2) "NoCollision")
  (Default|AddCollision _asbp_first_person_character (Variables|Default|GetBoxReturn_2)))

(event OnComponentEndOverlap(BoxReturn_1)
  (params (OverlappedComponent :type Primitive%20Component%20Object%20Reference) (OtherActor :type Actor%20Object%20Reference) (OtherComp :type Primitive%20Component%20Object%20Reference) (OtherBodyIndex :type Integer))
  (bind _asbp_first_person_character (Utilities|Casting|CastToBP_FirstPersonCharacter OtherActor))
  (Default|ReloadRooms _asbp_first_person_character)
  (Default|AddCollision _asbp_first_person_character (Variables|Default|GetBoxExit_3)))

(event OnComponentEndOverlap(BoxReturn_2)
  (params (OverlappedComponent :type Primitive%20Component%20Object%20Reference) (OtherActor :type Actor%20Object%20Reference) (OtherComp :type Primitive%20Component%20Object%20Reference) (OtherBodyIndex :type Integer))
  (bind _asbp_first_person_character (Utilities|Casting|CastToBP_FirstPersonCharacter OtherActor))
  (Default|ReloadRooms _asbp_first_person_character)
  (Default|AddCollision _asbp_first_person_character (Variables|Default|GetBoxExit_4)))

(event OnComponentEndOverlap(BoxReturn_3)
  (params (OverlappedComponent :type Primitive%20Component%20Object%20Reference) (OtherActor :type Actor%20Object%20Reference) (OtherComp :type Primitive%20Component%20Object%20Reference) (OtherBodyIndex :type Integer))
  (bind _asbp_first_person_character (Utilities|Casting|CastToBP_FirstPersonCharacter OtherActor))
  (Default|ReloadRooms _asbp_first_person_character))

(event OnComponentEndOverlap(BoxExit_3)
  (params (OverlappedComponent :type Primitive%20Component%20Object%20Reference) (OtherActor :type Actor%20Object%20Reference) (OtherComp :type Primitive%20Component%20Object%20Reference) (OtherBodyIndex :type Integer))
  (bind _asbp_first_person_character (Utilities|Casting|CastToBP_FirstPersonCharacter OtherActor))
  (Default|RespawnRooms _asbp_first_person_character _asbp_first_person_character self))

(event OnComponentEndOverlap(BoxExit_4)
  (params (OverlappedComponent :type Primitive%20Component%20Object%20Reference) (OtherActor :type Actor%20Object%20Reference) (OtherComp :type Primitive%20Component%20Object%20Reference) (OtherBodyIndex :type Integer))
  (bind _asbp_first_person_character (Utilities|Casting|CastToBP_FirstPersonCharacter OtherActor))
  (Default|RespawnRooms _asbp_first_person_character _asbp_first_person_character self))

(event EventBeginPlay)

(event Collision|EventActorBeginOverlap
  (params (OtherActor :type Actor%20Object%20Reference)))

(event EventTick
  (params (DeltaSeconds :type Float%20%28single-precision%29)))

(fn ConstructionScript)